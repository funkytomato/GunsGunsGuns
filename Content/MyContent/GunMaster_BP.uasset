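; GunMaster_BP is a first-person gun actor with its own Arms and a GunMesh snapped to the GripPoint socket at construction.
; FireProjectile expects a parent FirstPersonCharacter, spawns a projectile at BarrelRefPoint aimed along that character's camera rotation, and plays the fire montage on Arms.
; StartShooting and StopShooting only toggle IsFiring; nothing here reads that flag or calls FireProjectile.
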(event Custom|StartShooting
  (Variables|Default|SetIsFiring true))

(event Custom|StopShooting
  (Variables|Default|SetIsFiring false))

(fn ConstructionScript
  (Transformation|AttachComponentToComponent (Variables|Default|GetGunMesh) (Variables|Default|GetArms) "GripPoint" "SnapToTarget" "SnapToTarget" "SnapToTarget" true))

(fn FireProjectile
  (bind _asfirst_person_character (Utilities|Casting|CastToFirstPersonCharacter (Actor|GetParentActor)))
  (Game|SpawnActorfromClass "/Game/FirstPersonBP/Blueprints/FirstPersonProjectile.FirstPersonProjectile_C" (Math|Transform|MakeTransform (Transformation|GetWorldLocation (Variables|Default|GetBarrel_RefPoint)) (Transformation|GetWorldRotation (Variables|/Game/FirstPersonBP/Blueprints/FirstPersonCharacter.FirstPersonCharacter_C|GetFirstPersonCamera _asfirst_person_character)) "1,1,1") "AlwaysSpawn" 0 0)
  (Animation|Montage|MontagePlay (Components|SkeletalMesh|GetAnimInstance (Variables|Default|GetArms)) "/Game/FirstPerson/Animations/FirstPersonFire_Montage.FirstPersonFire_Montage" 1.0 "MontageLength" 0.0 true))